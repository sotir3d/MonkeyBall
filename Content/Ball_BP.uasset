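; Player-controlled rolling ball that moves by physics force, with a tilting camera that follows the input.
; RotateForward and RotateRight push the ball along its forward and right vectors, scaled by TiltForce.
; The same axes pitch and roll the SpringArm up to TiltMaxDegree, with pitch offset by CameraDefaultAngle.
; A second RotateRight handler also yaws the ball; Tick and CameraYaw are empty.
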(event EventTick
  (params (DeltaSeconds :type Float%20%28single-precision%29)))

(event Input|AxisEvents|InputAxisRotateForward
  (params (AxisValue :type Float%20%28single-precision%29))
  (bind _springarm (Variables|Default|GetSpringArm))
  (bind _ball (Variables|Default|GetBall))
  (bind _returnvalue (Transformation|GetWorldRotation _springarm))
  (bind (_roll _pitch _yaw) (Math|Rotator|BreakRotator _returnvalue))
  (Class|PrimitiveComponent|AddForceatLocation _ball (* (Math|Vector|GetForwardVector (Variables|Default|GetBall)) (* AxisValue (Variables|Default|GetTiltForce))) (Transformation|GetWorldLocation _ball) "None")
  (Transformation|SetWorldRotation (Variables|Default|GetSpringArm) (Math|Rotator|MakeRotator _roll (+ (* (Input|AxisValues|GetRotateForward) (Variables|Default|GetTiltMaxDegree)) (Variables|Default|GetCameraDefaultAngle)) _yaw) false false))

(event Input|AxisEvents|InputAxisCameraYaw
  (params (AxisValue :type Float%20%28single-precision%29)))

(event Input|AxisEvents|InputAxisRotateRight
  (params (AxisValue :type Float%20%28single-precision%29))
  (bind _ball (Variables|Default|GetBall))
  (bind _returnvalue (Transformation|GetWorldRotation _ball))
  (bind (_roll _pitch _yaw) (Math|Rotator|BreakRotator _returnvalue))
  (Transformation|SetWorldRotation (Variables|Default|GetBall) (Math|Rotator|MakeRotator _roll _pitch (+ _yaw (* AxisValue 2.0))) false false))

(event Input|AxisEvents|InputAxisRotateRight
  (params (AxisValue :type Float%20%28single-precision%29))
  (bind _ball (Variables|Default|GetBall))
  (bind _springarm (Variables|Default|GetSpringArm))
  (bind _returnvalue (Transformation|GetWorldRotation _springarm))
  (bind (_roll _pitch _yaw) (Math|Rotator|BreakRotator _returnvalue))
  (Class|PrimitiveComponent|AddForceatLocation _ball (* (Math|Vector|GetRightVector (Variables|Default|GetBall)) (* AxisValue (Variables|Default|GetTiltForce))) (Transformation|GetWorldLocation _ball) "None")
  (Transformation|SetWorldRotation (Variables|Default|GetSpringArm) (Math|Rotator|MakeRotator (* (Input|AxisValues|GetRotateRight) (Variables|Default|GetTiltMaxDegree) -1.0) _pitch _yaw) false false))

(fn ConstructionScript)